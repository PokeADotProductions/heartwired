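; BearOnlyTerrain is an environment hazard that periodically damages Talia while she stands inside its Box volume.
; When Talia enters, the overlap event starts a looping two-second timer, so damage begins only after the first interval.
; Each tick finds the first Talia in the level and sends her a TakeDamage message if still overlapping, otherwise it pauses the timer.
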(event `self.Box.OnComponentBeginOverlap`
  (params (OverlappedComponent :type "PrimitiveComponent Object Reference") (OtherActor :type "Actor Object Reference") (OtherComp :type "PrimitiveComponent Object Reference") (OtherBodyIndex :type Integer) (bFromSweep :type Boolean) (SweepResult :type "HitResult Structure (by ref)"))
  (cast `/Game/Blueprints/Character/Player/Talia/Talia` OtherActor)
  (bind _returnvalue (`KismetSystemLibrary.K2_SetTimerDelegate` (delegate `HurtTalia`) 2.0 true))
  (set `self.timerHandle` _returnvalue))

(event `HurtTalia`
  (bind _outactors (`GameplayStatics.GetAllActorsOfClass` "/Game/Blueprints/Character/Player/Talia/Talia.Talia_C"))
  (bind _output (`|GetArrayItem` _outactors))
  (if (`PrimitiveComponent.IsOverlappingActor` (`self.Box`) _output)
    (message `/Game/Blueprints/Character/Damageable.TakeDamage` _output 1.0)
    (else
      (`KismetSystemLibrary.K2_PauseTimerHandle` (`self.timerHandle`)))))

(fn `UserConstructionScript`)