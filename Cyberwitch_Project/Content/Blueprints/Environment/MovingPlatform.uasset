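; Moving platform actor that shuttles back and forth by a relative offset, starting automatically on BeginPlay.
; MoveTo and MoveBack use MoveComponentTo to shift the root by RelPosition over TimeLength, keeping rotation, then wait HoldDuration and call each other in an endless loop.
; Each leg also loops over attached actors, issuing the same relative offset move on their root components.
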(event `self.ReceiveBeginPlay`
  (`parent.ReceiveBeginPlay`)
  (`self.MoveTo`))

(event `MoveTo`
  (bind _defaultsceneroot (`self.DefaultSceneRoot`))
  (bind _returnvalue (`SceneComponent.GetRelativeTransform` _defaultsceneroot))
  ;[1 1 1] Move Self
  (`|ExecutionSequence`
    (:`then_0`
      (`KismetSystemLibrary.MoveComponentTo` _defaultsceneroot (+ (.location _returnvalue) (`self.relPosition`)) (`KismetMathLibrary.MakeRotator` (.roll (.rotation _returnvalue)) (.pitch (.rotation _returnvalue)) (.yaw (.rotation _returnvalue))) false false (`self.timeLength`) true)
      (`KismetSystemLibrary.Delay` (`self.holdDuration`))
      (`self.MoveBack`))
    (:`then_1`
      ;[1 1 1] Move all attached actors
      (for _array_element (`self.GetAttachedActors`)
        (bind _rootcomponent (`Actor.RootComponent` _array_element))
        (bind _returnvalue_2 (`SceneComponent.GetRelativeTransform` _rootcomponent))
        (`KismetSystemLibrary.MoveComponentTo` _rootcomponent (+ (.location _returnvalue_2) (`self.relPosition`)) (`KismetMathLibrary.MakeRotator` (.roll (.rotation _returnvalue_2)) (.pitch (.rotation _returnvalue_2)) (.yaw (.rotation _returnvalue_2))) false false (`self.timeLength`) true)))))

(event `MoveBack`
  (bind _defaultsceneroot (`self.DefaultSceneRoot`))
  (bind _returnvalue (`SceneComponent.GetRelativeTransform` _defaultsceneroot))
  ;[1 1 1] Undo Moves
  (`|ExecutionSequence`
    (:`then_0`
      (`KismetSystemLibrary.MoveComponentTo` _defaultsceneroot (- (.location _returnvalue) (`self.relPosition`)) (`KismetMathLibrary.MakeRotator` (.roll (.rotation _returnvalue)) (.pitch (.rotation _returnvalue)) (.yaw (.rotation _returnvalue))) false false (`self.timeLength`) true)
      (`KismetSystemLibrary.Delay` (`self.holdDuration`))
      (`self.MoveTo`))
    (:`then_1`
      (for _array_element (`self.GetAttachedActors`)
        (bind _rootcomponent (`Actor.RootComponent` _array_element))
        (bind _returnvalue_2 (`SceneComponent.GetRelativeTransform` _rootcomponent))
        (`KismetSystemLibrary.MoveComponentTo` _rootcomponent (- (.location _returnvalue_2) (`self.relPosition`)) (`KismetMathLibrary.MakeRotator` (.roll (.rotation _returnvalue_2)) (.pitch (.rotation _returnvalue_2)) (.yaw (.rotation _returnvalue_2))) false false (`self.timeLength`) true)))))

(fn `UserConstructionScript`
  (`parent.UserConstructionScript`))