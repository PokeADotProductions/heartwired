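; TutorialNextLevel is a trigger actor that moves the game from the tutorial to the next level.
; It keeps a count of overlapping actors, raised on begin overlap and lowered on end overlap, without filtering for players.
; When the count reaches one, it shows a LoadingScreen widget, waits briefly, then opens the level named by NextLevelName.
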(event `self.ReceiveActorBeginOverlap`
  (params (OtherActor :type "Actor Object Reference"))
  (bind _numofplayer (`self.numOfPlayer`))
  (`/Engine/EditorBlueprintResources/StandardMacros.IncrementInt` _numofplayer
    (:`  `
      (if (== _numofplayer 1)
        (bind _returnvalue (`|CreateWidget` "/Game/Blueprints/UI/LoadingScreen.LoadingScreen_C"))
        (`UserWidget.AddToViewport` _returnvalue 0)
        (`KismetSystemLibrary.Delay` 0.2)
        (`GameplayStatics.OpenLevel` (`self.NextLevelName`))))))

(event `self.ReceiveActorEndOverlap`
  (params (OtherActor :type "Actor Object Reference"))
  (`/Engine/EditorBlueprintResources/StandardMacros.DecrementInt` (`self.numOfPlayer`)))

(fn `UserConstructionScript`)