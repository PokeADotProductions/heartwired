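; Screen actor that switches the player's view when a BaseCharacter enters its Bounds volume.
; On BeginPlay it offsets its camera along Y by a distance derived from the bounds' extents and the camera's aspect ratio.
; On overlap it becomes the character's CurrentScreen, then SetCamera checks the controller state and blends the view to this fixed camera, or to the character if IsMoving is set.
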(event `self.ReceiveBeginPlay`
  (bind _camera (`self.Camera`))
  ;[1 1 1] Set Up Camera Position
  (bind _location (`self.CalcCameraPosition`))
  (`SceneComponent.K2_SetWorldLocation` _camera _location false true)
  (`SceneComponent.SetWorldScale3D` _camera (1.0 1.0 1.0)))

(event `self.bounds.OnComponentBeginOverlap`
  (params (OverlappedComponent :type "PrimitiveComponent Object Reference") (OtherActor :type "Actor Object Reference") (OtherComp :type "PrimitiveComponent Object Reference") (OtherBodyIndex :type Integer) (bFromSweep :type Boolean) (SweepResult :type "HitResult Structure (by ref)"))
  (bind _asbase_character (cast `/Game/Blueprints/Character/Player/BaseCharacter` OtherActor))
  (set `/Game/Blueprints/Character/Player/BaseCharacter.CurrentScreen` self _asbase_character)
  (`self.SetCamera` 0.5 _asbase_character))

(fn `CalcCameraPosition`
  (returns (location :type "Vector Structure"))
  (bind _bounds (`self.bounds`))
  (bind (_returnvalue_x _returnvalue_y _returnvalue_z) (`KismetMathLibrary.BreakVector` (`SceneComponent.K2_GetComponentLocation` _bounds)))
  (bind (_origin _boxextent) (`KismetSystemLibrary.GetComponentBounds` _bounds))
  (return (`KismetMathLibrary.MakeVector` _returnvalue_x (+ _returnvalue_y (`KismetMathLibrary.FMax` (.x _boxextent) (* (`CameraComponent.AspectRatio` (`self.Camera`)) (.z _boxextent)))) _returnvalue_z)))

(fn `SetCamera`
  (params (BlendTime :type "Float (double-precision)") (Character :type "/Game/Blueprints/Character/Player/BaseCharacter Object Reference"))
  (bind _asbase_controller (cast `/Game/Blueprints/Character/Player/BaseController` (`Pawn.GetController` Character)))
  (if (`|EnumEquality` (`/Game/Blueprints/Character/Player/BaseController.state` _asbase_controller) "NewEnumerator0")
    (if (`self.isMoving`)
      (`PlayerController.SetViewTargetWithBlend` (`GameplayStatics.GetPlayerController` 0) Character BlendTime "VTBlend_Linear" 0.0 true)
      (else
        (`PlayerController.SetViewTargetWithBlend` (`GameplayStatics.GetPlayerController` 0) self BlendTime "VTBlend_Linear" 0.0 true)))))

(fn `UserConstructionScript`)