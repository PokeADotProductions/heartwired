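; BaseCharacter is a character Blueprint that provides basic health tracking and death detection.
; CurrentHealth is set to MaxHealth in both the Construction Script and BeginPlay.
; The ChangeHealth event subtracts incoming damage without clamping, then calls Die when IsDead finds health at or below zero.
; The body of Die is not defined in these graphs, and overlap and Tick events are unused.
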(event `self.ChangeHealth`
  (params (DamageToBeDealt :type Integer) (Source :type "Actor Object Reference"))
  (set `self.CurrentHealth` (- (`self.CurrentHealth`) DamageToBeDealt))
  (bind _isdead (`self.IsDead`))
  (if _isdead
    (`self.Die`)))

(event `self.ReceiveBeginPlay`
  (set `self.CurrentHealth` (`self.MaxHealth`)))

(fn `IsDead`
  (returns (IsDead :type Boolean))
  (return (<= (`self.CurrentHealth`) 0)))

(fn `UserConstructionScript`
  (set `self.CurrentHealth` (`self.MaxHealth`)))